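; BP_leaderboard_data holds the data for one main menu leaderboard entry: position, username, run statistics and mode.
; Its single SetData function copies the incoming values into the asset's variables.
; Ghost kills, pills collected, deaths, level and level time are converted from integers to text, while position, username, hardcore mode and game mode are stored as passed.
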(fn SetData
  (params (position :type Integer) (username :type Text) (ghostKilled :type Integer) (pillCollected :type Integer) (playerDeaths :type Integer) (level :type Integer) (levelTime :type Integer) (hardcoreMode :type Boolean) (gameMode :type Text))
  (Variables|Default|SetLB_position position)
  (Variables|Default|SetUser username)
  (Variables|Default|SetGhostKilled (Utilities|Text|ToText(Integer) ghostKilled))
  (Variables|Default|SetPillsCollected (Utilities|Text|ToText(Integer) pillCollected))
  (Variables|Default|SetDeaths (Utilities|Text|ToText(Integer) playerDeaths))
  (Variables|Default|SetLevel (Utilities|Text|ToText(Integer) level))
  (Variables|Default|SetLevelTime (Utilities|Text|ToText(Integer) levelTime))
  (Variables|Default|SetHarcoreMode hardcoreMode)
  (Variables|Default|SetGameMode gameMode))